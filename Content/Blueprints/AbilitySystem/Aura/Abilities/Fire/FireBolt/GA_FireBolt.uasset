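; Fire Bolt gameplay ability that casts homing projectiles from the weapon at the player's aimed target.
; A forward trace supplies location and hit actor, then the ability commits, turns the avatar and plays the cast montage.
; A montage gameplay event triggers SpawnProjectiles, with pitch scaled by weapon-tip-to-target distance, and the ability ends when the montage finishes or is cut short.
; An older under-mouse targeting node remains unconnected.
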(event Ability|EventActivateAbility
  (bind _datahandle (|TargetDataForwardTrace 8e+03 3e+01 true)
    (:ValidData
      (Ability|CommitAbility)
      (Variables|Default|SetProjectileTargetLocation (.Location (Collision|BreakHitResult (Ability|TargetData|GetHitResultfromTargetData _datahandle))))
      (Variables|Default|SetMouseHitActor (.HitActor (Collision|BreakHitResult (Ability|TargetData|GetHitResultfromTargetData _datahandle))))
      (Class|CombatInterface|UpdateFacingTarget(Message) (Ability|GetAvatarActorfromActorInfo) (Variables|Default|GetProjectileTargetLocation))
      (|PlayMontageandWaitProxy "None" "/Game/Assets/Characters/Aura/Animations/Abilities/AM_Cast_FireBolt.AM_Cast_FireBolt" 1.0 "None" false 1.0 0.0 false
        (:then
          (Ability|Tasks|WaitGameplayEvent "(TagName=\"Event.Montage.FireBolt\")" 0
            (:EventReceived
              ;[0.3594 0.2344 0.02059 0.5] Hitting Close Targets with wider, slower spread of projectiles. CAN BE UPGRADED!!!!!!!!!
              (bind _returnvalue (Class|CombatInterface|GetWeapon(Message) (Ability|GetAvatarActorfromActorInfo)))
              (Class|AuraFireBolt|SpawnProjectiles (Variables|Default|GetProjectileTargetLocation) (GameplayTags|MakeLiteralGameplayTag "(TagName=\"CombatSocket.Weapon\")") false (- (* (/ (Math|Vector|Distance(Vector) (Variables|Default|GetProjectileTargetLocation) (Transformation|GetSocketLocation _returnvalue "TipSocket")) 6e+02) 5e+01) 2e+01) (Variables|Default|GetMouseHitActor)))))
        (:OnCompleted
          (Ability|EndAbility :!label _label))
        (:OnInterrupted
          (goto _label))
        (:OnCancelled
          (goto _label))))))