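; Melee attack gameplay ability that turns the avatar toward its combat target and plays a random montage from the character's attack list.
; Gameplay events matching the montage's tag collect unique hit actors, and each also starts a wait for Montage.Cancel.
; That cancel event damages every collected non-friendly actor and ends the ability.
; If the montage completes or is interrupted or cancelled first, the list clears without damage.
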(event Ability|EventActivateAbility
  (bind _returnvalue (Ability|GetAvatarActorfromActorInfo))
  (bind _returnvalue_2 (Class|EnemyInterface|GetCombatTarget(Message) _returnvalue))
  (bind _ascombat_interface (Utilities|Casting|CastToCombatInterface _returnvalue))
  (Class|CombatInterface|UpdateFacingTarget _ascombat_interface (Transformation|GetActorLocation _returnvalue_2))
  ;[1 1 1] Get a random attack from montages.
  (bind _returnvalue_3 (Class|CombatInterface|GetAttackMontages(Message) (Ability|GetAvatarActorfromActorInfo)))
  (if (Utilities|Array|IsNotEmpty _returnvalue_3)
    (bind _output_get (Variables|Default|SetTaggedMontage (.OutItem (Utilities|Array|Random _returnvalue_3))))
    (|PlayMontageandWaitProxy "None" (.Montage (Utilities|Struct|BreakTaggedMontage _output_get)) 1.0 "None" false 1.0 0.0 false
      (:then
        (bind _payload (Ability|Tasks|WaitGameplayEvent (.MontageTag (Utilities|Struct|BreakTaggedMontage _output_get)) 0)
          (:EventReceived
            (Utilities|Array|AddUnique (Variables|Default|GetHitActorList) (.Target (Utilities|Struct|BreakGameplayEventData _payload)))
            (Ability|Tasks|WaitGameplayEvent "(TagName=\"Montage.Cancel\")" 0
              (:EventReceived
                (for _array_element (Variables|Default|GetHitActorList)
                  (if (Class|AuraAbilitySystemLibrary|IsNotFriend (Ability|GetAvatarActorfromActorInfo) _array_element)
                    (Class|AuraDamageGameplayAbility|CauseDamage _array_element)))
                (Utilities|Array|Clear (Variables|Default|GetHitActorList))
                (Ability|EndAbility))))))
      (:OnCompleted
        (Utilities|Array|Clear (Variables|Default|GetHitActorList) :!label _label)
        (Ability|EndAbility))
      (:OnInterrupted
        (goto _label))
      (:OnCancelled
        (goto _label)))
    (else
      (Development|PrintString "ADD MONTAGES TO CHARACTER")
      (Ability|EndAbility))))

(event Ability|EventOnEndAbility
  (params (bWasCancelled :type Boolean)))