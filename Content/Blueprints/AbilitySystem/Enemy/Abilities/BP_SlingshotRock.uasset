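; BP_SlingshotRock is a rock projectile for an enemy slingshot ability, with no active logic in its own graphs.
; BeginPlay, Tick, overlap and the construction script are empty, so any flight or hit behavior is not defined here.
; Leftover disconnected nodes would randomize yaw, pitch and roll rates and spin RockMesh for a rolling look, but they never run.
; The author's note marks that spin logic as cheap but safe to delete.
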(event EventBeginPlay
  ;[0.15 0.15 0.15 0.5] This is for rolling projectile, doesn't cost much but still can be deleted!!
)

(event Collision|EventActorBeginOverlap
  (params (OtherActor :type Actor%20Object%20Reference)))

(event EventTick
  (params (DeltaSeconds :type Float%20%28single-precision%29))
  ;[0.15 0.15 0.15 0.5] This is for rolling projectile, doesn't cost much but still can be deleted!!
)

(fn ConstructionScript)