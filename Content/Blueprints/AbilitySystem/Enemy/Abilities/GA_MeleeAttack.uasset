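; Enemy melee attack Gameplay Ability that turns the avatar toward its combat target and plays a random tagged attack montage.
; Gameplay events with the montage's tag collect unique hit actors, then a Montage.End event triggers damage on the non-friendly ones.
; Each damaged actor also fires a MeleeImpact GameplayCue at the montage's combat socket.
; The ability clears the hit list and ends after processing or when the montage completes, is interrupted or is cancelled.
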(event Ability|EventActivateAbility
  (bind _returnvalue (Ability|GetAvatarActorfromActorInfo))
  (Variables|Default|SetHasHitTarget false)
  (bind _returnvalue_2 (Class|EnemyInterface|GetCombatTarget(Message) _returnvalue))
  (bind _ascombat_interface (Utilities|Casting|CastToCombatInterface _returnvalue))
  (Class|CombatInterface|UpdateFacingTarget _ascombat_interface (Transformation|GetActorLocation _returnvalue_2))
  ;[1 1 1] Get a random attack from montages
  (bind _returnvalue_3 (Class|CombatInterface|GetAttackMontages(Message) (Ability|GetAvatarActorfromActorInfo)))
  ;;[0.15 0.15 0.15 0.5] Do we really need to check?
  (if (Utilities|Array|IsNotEmpty _returnvalue_3)
    (bind _output_get (Variables|Default|SetTaggedMontage (.OutItem (Utilities|Array|Random _returnvalue_3))))
    (|PlayMontageandWaitProxy "None" (.Montage (Utilities|Struct|BreakTaggedMontage _output_get)) 1.0 "None" false 1.0 0.0 false
      (:then
        (bind _payload (Ability|Tasks|WaitGameplayEvent (.MontageTag (Utilities|Struct|BreakTaggedMontage _output_get)) 0)
          (:EventReceived
            (Utilities|Array|AddUnique (Variables|Default|GetHitActorList) (.Target (Utilities|Struct|BreakGameplayEventData _payload)))
            (Ability|Tasks|WaitGameplayEvent "(TagName=\"Montage.End\")" 0
              (:EventReceived
                ;[0.15 0.15 0.15 0.5] We use combat socket location for vfx and sfx
                (bind _returnvalue_4 (Class|CombatInterface|GetCombatSocketLocation(Message) (Ability|GetAvatarActorfromActorInfo) (.SocketTag (Utilities|Struct|BreakTaggedMontage (Variables|Default|GetTaggedMontage)))))
                (Variables|Default|SetCombatSocketLocation _returnvalue_4)
                (for _array_element (Variables|Default|GetHitActorList)
                  ;[0.15 0.15 0.15 0.5] Just for Debug
                  (Development|PrintText (Utilities|Text|ToText(String) (Utilities|GetDisplayName _array_element)))
                  (if (Class|AuraAbilitySystemLibrary|IsNotFriend (Ability|GetAvatarActorfromActorInfo) _array_element)
                    (Class|AuraDamageGameplayAbility|CauseDamage _array_element)
                    ;[0.15 0.15 0.15 0.5] OPTIMISATION: IF We are going to execute cue for each character got hit then remove this check, its pointless
                    (Variables|Default|SetHasHitTarget true)
                    (if (Variables|Default|GetHasHitTarget)
                      (bind _returnvalue_5 (Class|EnemyInterface|GetCombatTarget(Message) (Ability|GetAvatarActorfromActorInfo)))
                      (Class|GameplayAbility|ExecuteGameplayCuewithParams "(TagName=\"GameplayCue.MeleeImpact\")" (Ability|GameplayCue|MakeGameplayCueParameters :AggregatedSourceTags (GameplayTags|MakeGameplayTagContainerfromTag (.MontageTag (Utilities|Struct|BreakTaggedMontage (Variables|Default|GetTaggedMontage)))) :Location (Variables|Default|GetCombatSocketLocation) :EffectCauser (Ability|GetAvatarActorfromActorInfo) :SourceObject _returnvalue_5)))))
                (Utilities|Array|Clear (Variables|Default|GetHitActorList))
                (Ability|EndAbility))))))
      (:OnCompleted
        (Utilities|Array|Clear (Variables|Default|GetHitActorList) :!label _label)
        (Ability|EndAbility))
      (:OnInterrupted
        (goto _label))
      (:OnCancelled
        (goto _label)))))

(event Ability|EventOnEndAbility
  (params (bWasCancelled :type Boolean)))