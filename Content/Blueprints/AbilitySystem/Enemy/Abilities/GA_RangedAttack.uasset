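; Enemy ranged attack gameplay ability that fires a projectile at the owner's combat target.
; On activation it turns the avatar toward a valid combat target and plays a montage picked at random from its attack montages.
; The montage's gameplay event spawns the projectile from the tagged socket toward the target's current location, with optional pitch override.
; The ability ends when the montage completes, is interrupted or is cancelled.
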(event Ability|EventActivateAbility
  (bind _returnvalue (Ability|GetAvatarActorfromActorInfo))
  (bind _returnvalue_2 (Class|EnemyInterface|GetCombatTarget(Message) _returnvalue))
  (Utilities|Casting|CastToCombatInterface _returnvalue_2)
  (Class|CombatInterface|UpdateFacingTarget(Message) _returnvalue (Transformation|GetActorLocation _returnvalue_2))
  (bind _returnvalue_3 (Class|CombatInterface|GetAttackMontages(Message) (Ability|GetAvatarActorfromActorInfo)))
  ;[0.15 0.15 0.15 0.5] Do we really need to check?
  (if (Utilities|Array|IsNotEmpty _returnvalue_3)
    (|PlayMontageandWaitProxy "None" (.Montage (Utilities|Struct|BreakTaggedMontage (.OutItem (Utilities|Array|Random _returnvalue_3)))) 1.0 "None" false 1.0 0.0 false
      (:then
        (Ability|Tasks|WaitGameplayEvent (.MontageTag (Utilities|Struct|BreakTaggedMontage (.OutItem (Utilities|Array|Random _returnvalue_3)))) 0 true
          (:EventReceived
            (bind _returnvalue_4 (Class|EnemyInterface|GetCombatTarget(Message) (Ability|GetAvatarActorfromActorInfo)))
            (Class|AuraProjectileSpell|SpawnProjectile (Transformation|GetActorLocation _returnvalue_4) (.SocketTag (Utilities|Struct|BreakTaggedMontage (.OutItem (Utilities|Array|Random _returnvalue_3)))) (Variables|Default|GetShouldOverridePitch) (Variables|Default|GetPitchOverride)))))
      (:OnCompleted
        (Ability|EndAbility :!label _label))
      (:OnInterrupted
        (goto _label))
      (:OnCancelled
        (goto _label)))))

(event Ability|EventOnEndAbility
  (params (bWasCancelled :type Boolean)))